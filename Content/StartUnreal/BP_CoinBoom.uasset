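; BP_CoinBoom is a spinning hazard actor that damages the player and explodes when hit.
; Tick continuously rotates its Sphere component.
; When the Sphere's hit event involves BP_FirstPersonCharacter, it adds damage through BP_PlayerState, spawns a greatly scaled-up P_Explosion emitter and destroys itself.
; The emitter location uses the Sphere's relative location rather than its world position.
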(event `self.ReceiveTick`
  (params (DeltaSeconds :type "Float (single-precision)"))
  (`SceneComponent.K2_AddRelativeRotation` (`self.Sphere`) (struct :`Yaw` 2.0 :`Roll` 2.0) false false))

(event `self.Sphere.OnComponentBeginOverlap`
  (params (OverlappedComponent :type "PrimitiveComponent Object Reference") (OtherActor :type "Actor Object Reference") (OtherComp :type "PrimitiveComponent Object Reference") (OtherBodyIndex :type Integer) (bFromSweep :type Boolean) (SweepResult :type "HitResult Structure (by ref)")))

(event `self.ReceiveBeginPlay`)

(event `self.Sphere.OnComponentHit`
  (params (HitComponent :type "PrimitiveComponent Object Reference") (OtherActor :type "Actor Object Reference") (OtherComp :type "PrimitiveComponent Object Reference") (NormalImpulse :type "Vector Structure") (Hit :type "HitResult Structure (by ref)"))
  (bind _asbp_first_person_character (cast `/Game/FirstPerson/Blueprints/BP_FirstPersonCharacter` OtherActor))
  (bind _asbp_player_state (cast `/Game/ThirdPerson/Blueprints/BP_PlayerState` (`Pawn.PlayerState` _asbp_first_person_character)))
  (`/Game/ThirdPerson/Blueprints/BP_PlayerState.AddDamage` _asbp_player_state 10.0)
  (`GameplayStatics.SpawnEmitterAtLocation` "/Game/StarterContent/Particles/P_Explosion.P_Explosion" (`SceneComponent.RelativeLocation` (`self.Sphere`)) (struct) (100.0 100.0 100.0))
  (`self.K2_DestroyActor`))

(fn `UserConstructionScript`)