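; BP_Up_Down is an actor whose Cube component oscillates vertically between two height limits.
; Each Tick moves the Cube by a fixed relative Z step without sweep, so the speed depends on frame rate.
; The IsUp flag sets the direction and flips when the Cube's relative Z passes the upper or lower bound.
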(event `self.ReceiveTick`
  (params (DeltaSeconds :type "Float (single-precision)"))
  (bind _cube (`self.Cube`))
  (bind _cube_2 (`self.Cube`))
  (bind (_relativelocation_x _relativelocation_y _relativelocation_z) (`KismetMathLibrary.BreakVector` (`SceneComponent.RelativeLocation` _cube)))
  (bind (_relativelocation_x_2 _relativelocation_y_2 _relativelocation_z_2) (`KismetMathLibrary.BreakVector` (`SceneComponent.RelativeLocation` _cube_2)))
  (if (`self.IsUp`)
    (`SceneComponent.K2_AddRelativeLocation` _cube_2 (0.0 0.0 2.0) false false)
    (if (> _relativelocation_z_2 300.0)
      (set `self.IsUp` false))
    (else
      (`SceneComponent.K2_AddRelativeLocation` _cube (0.0 0.0 -2.0) false false)
      (if (< _relativelocation_z 0.0)
        (set `self.IsUp` true)))))

(fn `UserConstructionScript`)