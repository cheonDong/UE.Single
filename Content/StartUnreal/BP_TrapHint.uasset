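; BP_TrapHint is a trigger actor that signals every BP_TrapCube in the level when something enters or leaves its Box.
; Begin overlap sends IsVisionMessage and end overlap sends IsDivisionMessage, both after checking that each cube implements the BP_Division interface.
; Each overlap event gathers the cubes afresh with GetAllActorsOfClass and does not filter the overlapping actor.
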(event `self.Box.OnComponentBeginOverlap`
  (params (OverlappedComponent :type "PrimitiveComponent Object Reference") (OtherActor :type "Actor Object Reference") (OtherComp :type "PrimitiveComponent Object Reference") (OtherBodyIndex :type Integer) (bFromSweep :type Boolean) (SweepResult :type "HitResult Structure (by ref)"))
  (bind _outactors (`GameplayStatics.GetAllActorsOfClass` "/Game/StartUnreal/BP_TrapCube.BP_TrapCube_C"))
  (for _array_element _outactors
    (bind _asbp_trap_cube (cast `/Game/StartUnreal/BP_TrapCube` _array_element))
    (if (`KismetSystemLibrary.DoesImplementInterface` _asbp_trap_cube "/Game/StartUnreal/BP_Division.BP_Division_C")
      (message `/Game/StartUnreal/BP_Division.IsVision` _asbp_trap_cube))))

(event `self.Box.OnComponentEndOverlap`
  (params (OverlappedComponent :type "PrimitiveComponent Object Reference") (OtherActor :type "Actor Object Reference") (OtherComp :type "PrimitiveComponent Object Reference") (OtherBodyIndex :type Integer))
  (bind _outactors (`GameplayStatics.GetAllActorsOfClass` "/Game/StartUnreal/BP_TrapCube.BP_TrapCube_C"))
  (for _array_element _outactors
    (bind _asbp_trap_cube (cast `/Game/StartUnreal/BP_TrapCube` _array_element))
    (if (`KismetSystemLibrary.DoesImplementInterface` _asbp_trap_cube "/Game/StartUnreal/BP_Division.BP_Division_C")
      (message `/Game/StartUnreal/BP_Division.IsDivision` _asbp_trap_cube))))

(fn `UserConstructionScript`)