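; BP_MoveLeftRight is an actor that slides its Sphere back and forth along the local X axis.
; Each Tick steps a counter by a fixed amount, sets it as the sphere's relative X, and flips direction at either limit, so speed depends on frame rate.
; BP_EventComponent's DoPlay and DoStop dispatchers toggle whether it moves.
; The overlap event, construction script and MyFunction are empty.
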(event `self.ReceiveTick`
  (params (DeltaSeconds :type "Float (single-precision)"))
  (if (`self.IsPlay`)
    (if (`self.IsMoveRight`)
      ;[1 1 1] 오른쪽 이동
      (set `self.Count` (+ (`self.Count`) 1.0))
      (`SceneComponent.K2_SetRelativeLocation` (`self.Sphere`) (`KismetMathLibrary.MakeVector` (`self.Count`)) false false)
      (if (> (`self.Count`) 100.0)
        (set `self.IsMoveRight` false))
      (else
        ;[1 1 1] 왼쪽 이동
        (set `self.Count` (- (`self.Count`) 1.0))
        (`SceneComponent.K2_SetRelativeLocation` (`self.Sphere`) (`KismetMathLibrary.MakeVector` (`self.Count`)) false false)
        (if (< (`self.Count`) 0.0)
          (set `self.IsMoveRight` true))))))

(event `self.Sphere.OnComponentBeginOverlap`
  (params (OverlappedComponent :type "PrimitiveComponent Object Reference") (OtherActor :type "Actor Object Reference") (OtherComp :type "PrimitiveComponent Object Reference") (OtherBodyIndex :type Integer) (bFromSweep :type Boolean) (SweepResult :type "HitResult Structure (by ref)")))

(event `self.BP_EventComponent.EventDispatcher_DoPlay`
  (set `self.IsPlay` true))

(event `self.BP_EventComponent.EventDispatcher_DoStop`
  (set `self.IsPlay` false))

(fn `MyFunction`
  (params (NewParam :type Boolean)))

(fn `UserConstructionScript`)