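; BP_SwitchBox is a trigger switch that starts and stops every BP_EventComponent in the level through overlaps on its Cube component.
; Begin overlap prints the names involved and calls DoPlay on each component found; end overlap calls DoStop.
; Both events scan all actors with GetAllActorsOfClass and take one component per actor via GetComponentByClass, with no filter on the overlapping actor.
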(event `self.Cube.OnComponentBeginOverlap`
  (params (OverlappedComponent :type "PrimitiveComponent Object Reference") (OtherActor :type "Actor Object Reference") (OtherComp :type "PrimitiveComponent Object Reference") (OtherBodyIndex :type Integer) (bFromSweep :type Boolean) (SweepResult :type "HitResult Structure (by ref)"))
  (`KismetSystemLibrary.PrintString` (`KismetStringLibrary.Concat_StrStr` (`KismetSystemLibrary.GetDisplayName` OverlappedComponent) (`KismetSystemLibrary.GetDisplayName` OtherActor) (`KismetSystemLibrary.GetDisplayName` OtherComp)))
  (bind _outactors (`GameplayStatics.GetAllActorsOfClass` "/Script/Engine.Actor"))
  (for _array_element _outactors
    (bind _returnvalue (`self.GetComponentByClass` _array_element "/Game/StartUnreal/BP_EventComponent.BP_EventComponent_C"))
    (`/Engine/EditorBlueprintResources/StandardMacros.IsValid` _returnvalue
      (:`Is Valid`
        (`/Game/StartUnreal/BP_EventComponent.DoPlay` _returnvalue)))))

(event `self.Cube.OnComponentEndOverlap`
  (params (OverlappedComponent :type "PrimitiveComponent Object Reference") (OtherActor :type "Actor Object Reference") (OtherComp :type "PrimitiveComponent Object Reference") (OtherBodyIndex :type Integer))
  (bind _outactors (`GameplayStatics.GetAllActorsOfClass` "/Script/Engine.Actor"))
  (for _array_element _outactors
    (bind _returnvalue (`self.GetComponentByClass` _array_element "/Game/StartUnreal/BP_EventComponent.BP_EventComponent_C"))
    (`/Engine/EditorBlueprintResources/StandardMacros.IsValid` _returnvalue
      (:`Is Valid`
        (`/Game/StartUnreal/BP_EventComponent.DoStop` _returnvalue)))))

(fn `UserConstructionScript`)