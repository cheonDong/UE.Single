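; BP_Left_Right is an actor that shuttles its Cube component back and forth along its relative X axis.
; Each Tick applies a fixed relative offset in the direction set by IsMoveLeft, flipping that flag when the cube passes either bound.
; Movement has no sweep and is not scaled by delta time, so its speed depends on frame rate.
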(event `self.ReceiveBeginPlay`)

(event `self.ReceiveTick`
  (params (DeltaSeconds :type "Float (single-precision)"))
  (bind _cube (`self.Cube`))
  (bind _cube_2 (`self.Cube`))
  (bind _relativelocation_x (`KismetMathLibrary.BreakVector` (`SceneComponent.RelativeLocation` _cube)))
  (bind _relativelocation_x_2 (`KismetMathLibrary.BreakVector` (`SceneComponent.RelativeLocation` _cube_2)))
  (if (`self.IsMoveLeft`)
    (`SceneComponent.K2_AddRelativeLocation` _cube_2 (2.0 0.0 0.0) false false)
    (if (> _relativelocation_x_2 300.0)
      (set `self.IsMoveLeft` false))
    (else
      (`SceneComponent.K2_AddRelativeLocation` _cube (-2.0 0.0 0.0) false false)
      (if (< _relativelocation_x 0.0)
        (set `self.IsMoveLeft` true)))))

(fn `UserConstructionScript`)