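; BP_MoveRect is an actor that moves its Cube around a square path in the local XZ plane, one unit per tick.
; A MoveType enum state machine steps through right, up, left and down, switching when the horizontal or vertical counter passes its limit.
; Play and stop dispatchers on BP_EventComponent open and close a gate that controls the per-tick movement.
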(event `self.ReceiveTick`
  (params (DeltaSeconds :type "Float (single-precision)"))
  (`/Engine/EditorBlueprintResources/StandardMacros.Gate` true :!label _label
    (:`Exit`
      (switch `/Game/StartUnreal/EN_MoveType` (`self.MoveType`)
        (:`NewEnumerator0`
          (bind _returnvalue (`self.MoveRight`))
          (if _returnvalue
            (set `self.MoveType` "NewEnumerator1")))
        (:`NewEnumerator1`
          ;[1 1 1] 위쪽으로 이동
          (set `self.Count_UD` (+ (`self.Count_UD`) 1.0))
          (`SceneComponent.K2_SetRelativeLocation` (`self.Cube`) (`KismetMathLibrary.MakeVector` (`self.Count_LR`) 0.0 (`self.Count_UD`)) false false)
          (if (> (`self.Count_UD`) 100.0)
            (set `self.MoveType` "NewEnumerator2")))
        (:`NewEnumerator2`
          ;[1 1 1] 왼쪽으로 이동
          (set `self.Count_LR` (- (`self.Count_LR`) 1.0))
          (`SceneComponent.K2_SetRelativeLocation` (`self.Cube`) (`KismetMathLibrary.MakeVector` (`self.Count_LR`) 0.0 (`self.Count_UD`)) false false)
          (if (< (`self.Count_LR`) 0.0)
            (set `self.MoveType` "NewEnumerator3")))
        (:`NewEnumerator3`
          ;[1 1 1] 아래로 이동
          (set `self.Count_UD` (- (`self.Count_UD`) 1.0))
          (`SceneComponent.K2_SetRelativeLocation` (`self.Cube`) (`KismetMathLibrary.MakeVector` (`self.Count_LR`) 0.0 (`self.Count_UD`)) false false)
          (if (< (`self.Count_UD`) 0.0)
            (set `self.MoveType` "NewEnumerator0")))))))

(event `self.BP_EventComponent.EventDispatcher_DoPlay`
  (goto _label :!via `Open`))

(event `self.BP_EventComponent.EventDispatcher_DoStop`
  (goto _label :!via `Close`))

(fn `MoveRight`
  (returns (ReturnValue :type Boolean))
  ;[1 1 1] 오른쪽 이동
  (set `self.Count_LR` (+ (`self.Count_LR`) 1.0))
  (`SceneComponent.K2_SetRelativeLocation` (`self.Cube`) (`KismetMathLibrary.MakeVector` (`self.Count_LR`) 0.0 (`self.Count_UD`)) false false)
  (return (> (`self.Count_LR`) 100.0)))

(fn `UserConstructionScript`)